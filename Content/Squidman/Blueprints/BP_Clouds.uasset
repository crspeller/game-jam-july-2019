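; BP_Clouds is an actor that scatters a field of instanced meshes, named as clouds, when play begins.
; BeginPlay runs 1089 iterations, stepping NextLocation along X and wrapping to a new Y row at a fixed height past the X limit.
; Each step adds a world-space instance to one InstancedStaticMesh, with random offsets on all three axes to break up the grid.
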(event EventBeginPlay
  (for _index (range 1 1089)
    (Variables|Default|SetNextLocation (+ (Variables|Default|GetNextLocation) "1500.000000, 0, 0"))
    (if (>= (.x (Variables|Default|GetNextLocation)) 2.5e+04)
      (Variables|Default|SetNextLocation (Math|Vector|MakeVector -2.5e+04 (+ (.y (Variables|Default|GetNextLocation)) 1.5e+03) 1e+04)))
    (Class|InstancedStaticMeshComponent|AddInstanceWorldSpace (Variables|Default|GetInstancedStaticMesh) (Math|Transform|MakeTransform (Math|Vector|MakeVector (+ (.X (Math|Vector|BreakVector (Variables|Default|GetNextLocation))) (Math|Random|RandomFloatinRange -1e+03 1e+03)) (+ (.Y (Math|Vector|BreakVector (Variables|Default|GetNextLocation))) (Math|Random|RandomFloatinRange -1e+03 1e+03)) (+ (.Z (Math|Vector|BreakVector (Variables|Default|GetNextLocation))) (Math|Random|RandomFloatinRange -1e+03 1e+03)))))))

(fn ConstructionScript)