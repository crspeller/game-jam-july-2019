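; BP_Fog is a fog Blueprint that gradually thickens exponential height fog once play begins.
; A looping timer set on BeginPlay repeatedly raises the fog density by a small fixed step.
; The timer pauses itself through its stored handle once the density reaches an upper limit.
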(event Custom|IncreaseFog
  (bind _exponentialheightfog (Variables|Default|GetExponentialHeightFog))
  (Class|ExponentialHeightFogComponent|SetFogDensity _exponentialheightfog (+ (Variables|/Script/Engine.ExponentialHeightFogComponent|GetFogDensity _exponentialheightfog) 0.005))
  (if (>= (Variables|/Script/Engine.ExponentialHeightFogComponent|GetFogDensity (Variables|Default|GetExponentialHeightFog)) 5.0)
    (Utilities|Time|PauseTimerbyHandle (Variables|Default|GetFogTimerHandle))))

(event EventBeginPlay
  (bind _returnvalue (Utilities|Time|SetTimerbyEvent (delegate Custom|IncreaseFog) 0.1 true))
  (Variables|Default|SetFogTimerHandle _returnvalue))

(fn ConstructionScript)