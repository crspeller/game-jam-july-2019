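; Game mode for a squid-hunting game jam level, where all squid generators must be destroyed before a timer bar fills.
; On BeginPlay it adds the squid bar HUD and spawns the generators at random positions around the origin.
; A looping one-second timer fills the enemy bar and opens the GameOver level when full.
; SquidDeath lowers the count and player bar, then switches the HUD screen and shows the cursor when none remain.
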(event Custom|GameOver
  (Game|OpenLevel(byName) "GameOver"))

(event Custom|SquidDeath
  (bind _squidbarref (Variables|Default|GetSquidBarRef))
  (bind _playerbar (Variables|/Game/Squidman/Art/Widgets/BPW_SquidBar.BPW_SquidBar_C|GetPlayerBar _squidbarref))
  (Math|Integer|DecrementInt (Variables|Default|GetSquidCount)
    (:%20%20
      (Progress|SetPercent _playerbar (- (Variables|/Script/UMG.ProgressBar|GetPercent _playerbar) 0.1))
      (if (<= (Variables|Default|GetSquidCount) 0)
        (Class|WidgetSwitcher|SetActiveWidgetIndex (Variables|/Game/Squidman/Art/Widgets/BPW_SquidBar.BPW_SquidBar_C|GetScreenSwitcher (Variables|Default|GetSquidBarRef)) 1)
        (Variables|/Script/Engine.PlayerController|SetbShowMouseCursor (Game|GetPlayerController 0) true)))))

(event Custom|GameTimer
  (bind _squidbarref (Variables|Default|GetSquidBarRef))
  (bind _enemybar (Variables|/Game/Squidman/Art/Widgets/BPW_SquidBar.BPW_SquidBar_C|GetEnemyBar _squidbarref))
  (Progress|SetPercent _enemybar (+ (Variables|/Script/UMG.ProgressBar|GetPercent _enemybar) 0.01))
  (if (>= (Variables|/Script/UMG.ProgressBar|GetPercent (Variables|/Game/Squidman/Art/Widgets/BPW_SquidBar.BPW_SquidBar_C|GetEnemyBar (Variables|Default|GetSquidBarRef))) 1.0)
    (CallFunction|GameOver)))

(event EventBeginPlay
  (bind _returnvalue (UserInterface|CreateWidget "/Game/Squidman/Art/Widgets/BPW_SquidBar.BPW_SquidBar_C" (Game|GetPlayerController 0)))
  (bind _output_get (Variables|Default|SetSquidBarRef _returnvalue))
  (UserInterface|Viewport|AddtoViewport _output_get 0)
  (for _index (range 1 10)
    (Variables|Default|SetRandomX (Math|Random|RandomFloatinRange 5e+03 2e+04))
    (if (Math|Random|RandomBool)
      _
      (else
        (Math|Float|NegateFloat (Variables|Default|GetRandomX)
          (:%20%20
            _))))
    (Variables|Default|SetRandomY (Math|Random|RandomFloatinRange 5e+03 2e+04))
    (if (Math|Random|RandomBool)
      _
      (else
        (Math|Float|NegateFloat (Variables|Default|GetRandomY)
          (:%20%20
            _))))
    (bind _returnvalue_2 (Game|SpawnActorfromClass "/Game/Squidman/Blueprints/BP_SquidGenerator.BP_SquidGenerator_C" (Math|Transform|MakeTransform (Math|Vector|MakeVector (Variables|Default|GetRandomX) (Variables|Default|GetRandomY) (Math|Random|RandomFloatinRange 0.0 8.5e+03)) "0, 0, 0" "1,1,1") "Undefined" 0 0))
    (bind _output_get_2 (Variables|Default|SetNewSquid _returnvalue_2))
    (Utilities|Array|Add (Variables|Default|GetSquidArray) _output_get_2)
    (Math|Integer|IncrementInt (Variables|Default|GetSquidCount)))
  (Utilities|Time|SetTimerbyEvent (delegate Custom|GameTimer) 1.0 true))

(event EventTick
  (params (DeltaSeconds :type Float%20%28single-precision%29)))

(fn ConstructionScript)