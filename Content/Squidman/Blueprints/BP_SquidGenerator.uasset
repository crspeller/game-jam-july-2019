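; Squid generator actor that bobs and glows, and reports a squid death to the July game jam game mode when any actor overlaps it, then destroys itself after a brief delay.
; A timeline supplies an alpha that a looping timer, rather than Tick, applies to the height offset from its starting elevation and to the glow of a dynamic radioactive-green material.
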(event Custom|EventBob
  (bind _returnvalue (Transformation|GetActorLocation))
  (Transformation|SetActorLocation (Math|Vector|MakeVector (.x _returnvalue) (.y _returnvalue) (Math|Float|Lerp (Variables|Default|GetOriginalElevation) (+ (Variables|Default|GetOriginalElevation) (Variables|Default|GetElevationAmount)) (Variables|Default|GetElevationAlpha))) false false)
  (Rendering|Material|SetScalarParameterValueonMaterials (Variables|Default|GetStaticMesh) "GlowAmount" (* (Variables|Default|GetElevationAlpha) 25.0)))

(event EventBeginPlay
  (bind _asbp_game_jam_july_game_mode (Utilities|Casting|CastToBP_GameJamJulyGameMode (Game|GetGameMode)))
  (Variables|Default|SetGameModeRef _asbp_game_jam_july_game_mode)
  (bind _returnvalue (Rendering|Material|CreateDynamicMaterialInstance "/Game/Squidman/Art/Materials/M_RadioactiveGreen.M_RadioactiveGreen" "None" :!class /Script/Engine.KismetMaterialLibrary))
  (Rendering|Material|SetMaterial (Variables|Default|GetStaticMesh) 3 _returnvalue)
  (Variables|Default|SetOriginalElevation (.z (Transformation|GetActorLocation)))
  (Utilities|Time|SetTimerbyEvent (delegate Custom|EventBob) 0.1 true)
  (bind _lerp (Timeline|BobbingTimeline Play)
    (:Update
      (Variables|Default|SetElevationAlpha _lerp))))

(event Collision|EventActorBeginOverlap
  (params (OtherActor :type Actor%20Object%20Reference))
  (Default|SquidDeath (Variables|Default|GetGameModeRef))
  (Utilities|FlowControl|Delay 0.1)
  (Actor|DestroyActor))

(event EventTick
  (params (DeltaSeconds :type Float%20%28single-precision%29)))

(fn ConstructionScript)